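; Projectile actor that flies along its local Velocity each tick and destroys enemies it overlaps.
; Overlapping an Enemy calls its DestroySelf, then the projectile destroys itself and spawns a Niagara impact effect.
; It ignores the player and tunnel but bursts the same way on any other actor.
; A construction-script lifespan removes stray shots, and a separate DestroySelf function repeats the burst logic.
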(event EventBeginPlay)

(event Collision|EventActorBeginOverlap
  (params (OtherActor :type Actor%20Object%20Reference))
  (bind _asenemy (Utilities|Casting|CastToEnemy OtherActor)
    (:then
      (Default|DestroySelf _asenemy))
    (:CastFailed
      (Utilities|Casting|CastToBP_Player OtherActor
        (:CastFailed
          (Utilities|Casting|CastToBP_Tunnel OtherActor
            (:CastFailed
              _))))))
  (Actor|DestroyActor)
  (Niagara|SpawnSystematLocation "/Game/InfiniteMatrix/Blueprints/Projectile_VFX.Projectile_VFX" (Transformation|GetActorLocation) "90.000000,0.000000,0.000000"))

(event EventTick
  (params (DeltaSeconds :type Float%20%28single-precision%29))
  (Transformation|AddActorLocalOffset (* (Variables|Default|GetVelocity) DeltaSeconds) false false))

(fn ConstructionScript
  (Actor|SetLifeSpan 4.0))

(fn DestroySelf
  (Actor|DestroyActor)
  (Niagara|SpawnSystematLocation "/Game/InfiniteMatrix/Blueprints/Projectile_VFX.Projectile_VFX" (Transformation|GetActorLocation) "90.000000,0.000000,0.000000"))
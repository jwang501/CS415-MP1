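; Enemy actor that awards score when shot and damages the player on collision.
; A Projectile overlap adds to BP_Player's score and destroys the enemy.
; A mesh hit on the player cuts health, then either triggers death and the restart display or slows forward speed with a minimum floor, and destroys the enemy.
; DestroySelf, not called within this file, also awards score, destroys the actor and spawns a destruction VFX.
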(event OnComponentHit(StaticMesh)
  (params (HitComponent :type Primitive%20Component%20Object%20Reference) (OtherActor :type Actor%20Object%20Reference) (OtherComp :type Primitive%20Component%20Object%20Reference) (NormalImpulse :type Vector :default "0, 0, 0") (Hit :type Hit%20Result%20Structure%20%28by%20ref%29))
  (bind _asbp_player (Utilities|Casting|CastToBP_Player OtherActor))
  (bind _output_get (Variables|/Game/InfiniteMatrix/Blueprints/BP_Player.BP_Player_C|SetHealth _asbp_player (- (Variables|/Game/InfiniteMatrix/Blueprints/BP_Player.BP_Player_C|GetHealth _asbp_player) 2)))
  (if (<= _output_get 0)
    (Variables|/Game/InfiniteMatrix/Blueprints/BP_Player.BP_Player_C|SetIsDead _asbp_player true)
    (Default|DisplayRestart _asbp_player)
    (else
      (Variables|/Game/InfiniteMatrix/Blueprints/BP_Player.BP_Player_C|SetForwardSpeed _asbp_player (Math|Float|Max(Float) (* (Variables|/Game/InfiniteMatrix/Blueprints/BP_Player.BP_Player_C|GetForwardSpeed _asbp_player) 0.5) 2e+03))))
  (Actor|DestroyActor))

(event EventBeginPlay)

(event Collision|EventActorBeginOverlap
  (params (OtherActor :type Actor%20Object%20Reference))
  (Utilities|Casting|CastToProjectile OtherActor)
  (bind _returnvalue (Actor|GetActorOfClass "/Game/InfiniteMatrix/Blueprints/BP_Player.BP_Player_C"))
  (Variables|/Game/InfiniteMatrix/Blueprints/BP_Player.BP_Player_C|SetScore _returnvalue (+ (Variables|/Game/InfiniteMatrix/Blueprints/BP_Player.BP_Player_C|GetScore _returnvalue) 1))
  (Actor|DestroyActor))

(event EventTick
  (params (DeltaSeconds :type Float%20%28single-precision%29)))

(fn ConstructionScript)

(fn DestroySelf
  (bind _returnvalue (Actor|GetActorOfClass "/Game/InfiniteMatrix/Blueprints/BP_Player.BP_Player_C"))
  (Variables|/Game/InfiniteMatrix/Blueprints/BP_Player.BP_Player_C|SetScore _returnvalue (+ (Variables|/Game/InfiniteMatrix/Blueprints/BP_Player.BP_Player_C|GetScore _returnvalue) 1))
  (Actor|DestroyActor)
  (Niagara|SpawnSystematLocation "/Game/InfiniteMatrix/Blueprints/Enemy_Destroy_VFX.Enemy_Destroy_VFX" (Transformation|GetActorLocation) "90.000000,0.000000,0.000000"))
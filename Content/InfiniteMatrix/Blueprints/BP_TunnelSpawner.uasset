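; Spawner actor that builds the tunnel course, chaining randomized-wall BP_Tunnel segments from the player's location.
; On BeginPlay it clears existing tunnels and spawns a starting chain, each segment placed at the newest one's SpawnPoint.
; Each chained segment randomly adds health packs and enemies at offsets ahead, meant to fall within a circular cross-section.
; CleanUp destroys enemies, clearing health packs inside that same loop.
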(event EventBeginPlay
  (CallFunction|SpawnIntialTunnels))

(event Collision|EventActorBeginOverlap
  (params (OtherActor :type Actor%20Object%20Reference)))

(event EventTick
  (params (DeltaSeconds :type Float%20%28single-precision%29)))

(fn ConstructionScript)

(fn SpawnTunnel
  (params (SpawnLocation :type Vector))
  (bind _returnvalue (Game|SpawnActorfromClass "/Game/InfiniteMatrix/Blueprints/BP_Tunnel.BP_Tunnel_C" (Math|Transform|MakeTransform SpawnLocation "0, 0, 0" "1.000000,1.000000,1.000000") "Undefined" "MultiplyWithRoot" 0 0))
  (bind _output_get (Variables|Default|SetNewestTunnel _returnvalue))
  (Variables|/Game/InfiniteMatrix/Blueprints/BP_Tunnel.BP_Tunnel_C|SetTunnel%20Spawner _output_get self)
  (Default|RandomizeWall _output_get))

(fn SpawnTunnelatSpawnPoint
  (bind _newesttunnel (Variables|Default|GetNewestTunnel))
  (bind _spawnpoint (Variables|/Game/InfiniteMatrix/Blueprints/BP_Tunnel.BP_Tunnel_C|GetSpawnPoint _newesttunnel))
  (bind _returnvalue (Transformation|GetWorldLocation _spawnpoint))
  (CallFunction|SpawnTunnel _returnvalue)
  (if (> (Math|Random|RandomInteger 10) 7)
    (CallFunction|SpawnHealthPack _returnvalue))
  (if (> (Math|Random|RandomInteger 10) 3)
    (CallFunction|SpawnEnemy _returnvalue)))

(fn SpawnIntialTunnels
  (Utilities|FlowControl|Sequence
    (:then_0
      (bind _outactors (Actor|GetAllActorsOfClass "/Game/InfiniteMatrix/Blueprints/BP_Tunnel.BP_Tunnel_C"))
      (for _array_element _outactors
        (Actor|DestroyActor _array_element)))
    (:then_1
      (for _index (range 0 2)
        (Utilities|IsValid (Variables|Default|GetNewestTunnel)
          (:Is%20Valid
            (CallFunction|SpawnTunnelatSpawnPoint))
          (:Is%20Not%20Valid
            (CallFunction|SpawnTunnel (Transformation|GetActorLocation (Game|Player|GetPlayerPawn 0)))))))))

(fn SpawnHealthPack
  (params (Origin :type Vector))
  (bind _returnvalue (Math|Random|RandomFloatinRange -4e+02 4e+02))
  (bind _returnvalue_2 (Math|Float|Square 4e+02))
  (bind _returnvalue_3 (Math|Float|Square _returnvalue))
  (bind _returnvalue_4 (- _returnvalue_2 _returnvalue_3))
  (bind _returnvalue_5 (Math|Float|Sqrt _returnvalue_4))
  (Game|SpawnActorfromClass "/Game/InfiniteMatrix/Blueprints/Health_Pack.Health_Pack_C" (Math|Transform|MakeTransform (+ Origin (Math|Vector|MakeVector (Math|Random|RandomFloatinRange 4e+02 2e+03) _returnvalue (Math|Random|RandomFloatinRange (* _returnvalue_5 -1.0) _returnvalue_5))) "0, 0, 0" "1.000000,1.000000,1.000000") "AdjustIfPossibleButDontSpawnIfColliding" "MultiplyWithRoot" 0 0))

(fn SpawnEnemy
  (params (Origin :type Vector))
  (bind _returnvalue (Math|Random|RandomFloatinRange -3.5e+02 3.5e+02))
  (bind _returnvalue_2 (Math|Float|Square 3.5e+02))
  (bind _returnvalue_3 (Math|Float|Square _returnvalue))
  (bind _returnvalue_4 (- _returnvalue_2 _returnvalue_3))
  (bind _returnvalue_5 (Math|Float|Sqrt _returnvalue_4))
  (Game|SpawnActorfromClass "/Game/InfiniteMatrix/Blueprints/Enemy.Enemy_C" (Math|Transform|MakeTransform (+ Origin (Math|Vector|MakeVector (Math|Random|RandomFloatinRange 1e+03 2.3e+03) _returnvalue (Math|Random|RandomFloatinRange (* _returnvalue_5 -1.0) _returnvalue_5))) "0, 0, 0" "1.000000,1.000000,1.000000") "AdjustIfPossibleButDontSpawnIfColliding" "MultiplyWithRoot" 0 0))

(fn CleanUp
  (bind _outactors (Actor|GetAllActorsOfClass "/Game/InfiniteMatrix/Blueprints/Enemy.Enemy_C"))
  (for _array_element _outactors
    (Actor|DestroyActor _array_element)
    (bind _outactors_2 (Actor|GetAllActorsOfClass "/Game/InfiniteMatrix/Blueprints/Health_Pack.Health_Pack_C"))
    (for _array_element_2 _outactors_2
      (Actor|DestroyActor _array_element_2))))